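; Lobby game mode for a networked game that manages joining players, character selection and match start.
; PostLogin registers players and sets up their lobby menu, or queues those over capacity for a timed kick.
; UpdateClients pushes player info, character availability and settings-window kick list updates, and computes CanStart from character and ready status.
; It also respawns chosen characters at random PlayerStarts, relays map settings, frees characters on logout and server-travels to the selected map.
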(event Custom|KickExtraPlayers
  (for _array_element (Variables|Default|GetExtraPlayers)
    (Utilities|IsValid _array_element
      (:Is%20Valid
        (bind _asbp_lobby_player_cronller (Utilities|Casting|CastToBP_LobbyPlayerCronller _array_element))
        (Default|Kicked _asbp_lobby_player_cronller "Host is FUll")))))

(event Custom|SwapCharacter
  (params (PlayerController :type Player%20Controller%20Object%20Reference) (CharacterClass :type BP%20Base%20Character%20Class%20Reference))
  (bind _returnvalue (Pawn|GetControlledPawn PlayerController))
  (bind _spawnpoints (Variables|Default|GetSpawnPoints))
  (Utilities|IsValid _returnvalue
    (:Is%20Valid
      (Actor|DestroyActor _returnvalue))
    (:Is%20Not%20Valid
      _))
  (bind _returnvalue_2 (Game|SpawnActorfromClass CharacterClass (Transformation|GetActorTransform (Utilities|Array|Get(acopy) _spawnpoints (Math|Random|RandomIntegerinRange 0 (- (Utilities|Array|Length _spawnpoints) 1)))) "Undefined" 0 0))
  (Pawn|Possess PlayerController _returnvalue_2))

(event Custom|UpdateKickList
  (bind _asbp_lobby_player_cronller (Utilities|Casting|CastToBP_LobbyPlayerCronller (Game|GetPlayerController 0)))
  (Utilities|IsValid (Variables|/Game/NetworkGame/BluePrints/Lobby/BP_LobbyPlayerCronller.BP_LobbyPlayerCronller_C|GetLobbyMenuRef _asbp_lobby_player_cronller)
    (:Is%20Valid
      (if (Widget|IsVisible (Variables|/Game/NetworkGame/BluePrints/Wigets/Lobby/WBP_LobbyMenu.WBP_LobbyMenu_C|GetGameSettingsWindow (Variables|/Game/NetworkGame/BluePrints/Lobby/BP_LobbyPlayerCronller.BP_LobbyPlayerCronller_C|GetLobbyMenuRef _asbp_lobby_player_cronller)))
        (Default|UpdatePlayerList (Variables|/Game/NetworkGame/BluePrints/Wigets/Lobby/WBP_LobbyMenu.WBP_LobbyMenu_C|GetGameSettingsWindow (Variables|/Game/NetworkGame/BluePrints/Lobby/BP_LobbyPlayerCronller.BP_LobbyPlayerCronller_C|GetLobbyMenuRef _asbp_lobby_player_cronller)))))))

(event Custom|UpdateClients
  (bind _connectedplayers (Variables|Default|GetConnectedPlayers))
  (bind _output_get (Variables|Default|SetCurrentPlayer (Utilities|Array|Length (Variables|Default|GetConnectedPlayers))))
  (if (> _output_get 0)
    (Utilities|Array|Clear (Variables|Default|GetConnectedPlayers))
    (for _array_element _connectedplayers
      (bind _asbp_lobby_player_cronller (Utilities|Casting|CastToBP_LobbyPlayerCronller _array_element))
      (Utilities|Array|Add (Variables|Default|GetConnectedPlayersInfo) (Variables|/Game/NetworkGame/BluePrints/Lobby/BP_LobbyPlayerCronller.BP_LobbyPlayerCronller_C|GetPlayerInfo _asbp_lobby_player_cronller))
      (Default|UpdatePlayerNumDisplayText _asbp_lobby_player_cronller (Variables|Default|GetCurrentPlayer) (Variables|Default|GetMaxPlayer)))
    (for _array_element_2 _connectedplayers
      (bind _asbp_lobby_player_cronller_2 (Utilities|Casting|CastToBP_LobbyPlayerCronller _array_element_2))
      (Default|UpdatePlayerInfoList _asbp_lobby_player_cronller_2 (Variables|Default|GetConnectedPlayersInfo))
      (Default|UpdateAvailableCharacters _asbp_lobby_player_cronller_2 (Variables|Default|GetAvailableCharacters))
      (CallFunction|UpdateKickList))
    (bind _array_element_3 (Utilities|Array|ForEachLoopwithBreak (Variables|Default|GetConnectedPlayersInfo) :!label _label)
      (:LoopBody
        (if (or (== (.characterclass _array_element_3) "/Game/NetworkGame/BluePrints/Character/BP_BaseCharacter.BP_BaseCharacter_C") (Utilities|Enum|Equal(Enum) (.readystatus _array_element_3) "NewEnumerator1"))
          (Variables|Default|SetCanStart false)
          (goto _label Break)
          (else
            (Variables|Default|SetCanStart true)))))))

(event Custom|StartGame
  (bind _returnvalue (Game|GetPlayerController 0))
  (Variables|/Game/NetworkGame/BluePrints/General/BP_GameInstance.BP_GameInstance_C|SetMapTime (.AsBP%20Game%20Instance (Utilities|Casting|CastToBP_GameInstance (Game|GetGameInstance))) (Variables|Default|GetMap%20Time))
  (switch int (Variables|Default|GetMapID)
    (:0
      (Development|ExecuteConsoleCommand "servertravel /Game/NetworkGame/Maps/Map01" _returnvalue))
    (:1
      (Development|ExecuteConsoleCommand "servertravel /Game/NetworkGame/Maps/Map02" _returnvalue))))

(event Custom|UpdateGameSettings
  (params (MapImage :type Texture%202D%20Object%20Reference) (MapName :type Text) (MapTime :type Text) (MapID :type Integer))
  (Variables|Default|SetMap%20Image MapImage)
  (Variables|Default|SetMap%20Name MapName)
  (Variables|Default|SetMap%20Time MapTime)
  (Variables|Default|SetMapID MapID)
  (for _array_element (Variables|Default|GetConnectedPlayers)
    (bind _asbp_lobby_player_cronller (Utilities|Casting|CastToBP_LobbyPlayerCronller _array_element))
    (Default|UpdateLobbySettings _asbp_lobby_player_cronller (Variables|Default|GetMap%20Image) (Variables|Default|GetMap%20Name) (Variables|Default|GetMap%20Time))))

(event Custom|KickPlayer
  (params (PlayerIndex :type Integer))
  (bind _asbp_lobby_player_cronller (Utilities|Casting|CastToBP_LobbyPlayerCronller (Utilities|Array|Get(acopy) (Variables|Default|GetConnectedPlayers) PlayerIndex)))
  (Default|Kicked _asbp_lobby_player_cronller "you got kicked"))

(event EventOnLogout
  (params (ExitingController :type Controller%20Object%20Reference))
  (bind _connectedplayers (Variables|Default|GetConnectedPlayers))
  (bind _as玩家控制器 (Utilities|Casting|CastToPlayerController ExitingController))
  (bind _asbp_lobby_player_cronller (Utilities|Casting|CastToBP_LobbyPlayerCronller (Utilities|Array|Get(acopy) _connectedplayers (Utilities|Array|FindItem _connectedplayers _as玩家控制器))))
  (Utilities|Array|SetArrayElem (Variables|Default|GetAvailableCharacters) (Variables|/Game/NetworkGame/BluePrints/Lobby/BP_LobbyPlayerCronller.BP_LobbyPlayerCronller_C|GetCurrentSelectCharacterIndex _asbp_lobby_player_cronller) true)
  (Utilities|Array|RemoveIndex (Variables|Default|GetConnectedPlayers) (Utilities|Array|FindItem _connectedplayers _as玩家控制器))
  (Utilities|Array|RemoveIndex (Variables|Default|GetConnectedPlayersInfo) (Utilities|Array|FindItem _connectedplayers _as玩家控制器))
  (CallFunction|UpdateClients))

(event EventPostLogin
  (params (NewPlayer :type Player%20Controller%20Object%20Reference))
  (bind _returnvalue (Game|GetGameInstance))
  (bind _asbp_game_instance (Utilities|Casting|CastToBP_GameInstance _returnvalue))
  (if (and (>= (Variables|Default|GetCurrentPlayer) (Variables|Default|GetMaxPlayer)) (!= (Variables|Default|GetMaxPlayer) 0))
    (Utilities|Array|Add (Variables|Default|GetExtraPlayers) NewPlayer)
    (Utilities|Time|SetTimerbyEvent (delegate Custom|KickExtraPlayers) 2.0 true)
    (else
      (Utilities|Array|Add (Variables|Default|GetConnectedPlayers) NewPlayer)
      (Variables|Default|SetMaxPlayer (Variables|/Game/NetworkGame/BluePrints/General/BP_GameInstance.BP_GameInstance_C|GetMaxPlayer _asbp_game_instance))
      (Variables|Default|SetServerName (Variables|/Game/NetworkGame/BluePrints/General/BP_GameInstance.BP_GameInstance_C|GetServerName _asbp_game_instance))
      (if (== (Utilities|Array|Length (Variables|Default|GetSpawnPoints)) 0)
        (bind _outactors (Actor|GetAllActorsOfClass "/Script/Engine.PlayerStart"))
        (Variables|Default|SetSpawnPoints _outactors))
      (bind _asbp_lobby_player_cronller (Utilities|Casting|CastToBP_LobbyPlayerCronller NewPlayer))
      (Default|InitialPlayerInfo _asbp_lobby_player_cronller)
      (Default|CreateLobbyMenu _asbp_lobby_player_cronller (Variables|Default|GetServerName))
      (Default|UpdateLobbySettings _asbp_lobby_player_cronller (Variables|Default|GetMap%20Image) (Variables|Default|GetMap%20Name) (Variables|Default|GetMap%20Time))
      (CallFunction|UpdateClients))))

(fn ConstructionScript)
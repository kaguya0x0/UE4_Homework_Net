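; Main menu GameMode that opens the menu screens and starts hosting or joining of network sessions.
; Show events create and add the main, host, server and option widgets, while the loading screen and error messages are delegated to BP_GameInstance1.
; Hosting stores server name and player limit in the GameInstance, creates a session and opens Lobby as a listen server.
; A failed join shows an error and rebuilds the main menu.
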(event Custom|ShowServerMenu
  (bind _returnvalue (UserInterface|CreateWidget "/Game/MultiplayerGame/Blueprints/Widget/MainMenu/7.7_C" (Game|GetPlayerController 0)))
  (UserInterface|Viewport|AddtoViewport _returnvalue 0))

(event Custom|ShowOptionMenu
  (bind _returnvalue (UserInterface|CreateWidget "/Game/NetworkGame/BluePrints/Wigets/MainMunu/WBP_OptionMenu.WBP_OptionMenu_C" (Game|GetPlayerController 0)))
  (UserInterface|Viewport|AddtoViewport _returnvalue 0))

(event Custom|HostGame
  (params (ServerName :type Text) (MaxPlayer :type Integer) (UseLAN :type Boolean))
  (bind _returnvalue (Game|GetGameInstance))
  (bind _asbp_game_instance_1 (Utilities|Casting|CastToBP_GameInstance1 _returnvalue))
  (Variables|/Game/MultiplayerGame/Blueprints/General/BP_GameInstance1.BP_GameInstance1_C|SetServerName _asbp_game_instance_1 ServerName)
  (Variables|/Game/MultiplayerGame/Blueprints/General/BP_GameInstance1.BP_GameInstance1_C|SetMaxPlayer _asbp_game_instance_1 MaxPlayer)
  (CallFunction|ShowLoadingScreen)
  (|Session (Game|GetPlayerController 0) MaxPlayer UseLAN
    (:OnSuccess
      (Game|OpenLevel(byName) "Lobby" true "listen"))
    (:OnFailure
      (Default|ShowMessageWindow _asbp_game_instance_1 "Failed to Create Session. Please Try Again."))))

(event Custom|JoinGame
  (params (Session :type Blueprint%20Session%20Result%20Structure))
  (CallFunction|ShowLoadingScreen)
  (|JoinSession (Game|GetPlayerController 0) Session
    (:OnFailure
      (Default|ShowMessageWindow (.AsBP%20Game%20Instance%201 (Utilities|Casting|CastToBP_GameInstance1 (Game|GetGameInstance))) "Failed to Join Session. Please Try Again.")
      (Viewport|RemoveAllWidgets)
      (CallFunction|ShowMainMenu))))

(event Custom|ShowLoadingScreen
  (Default|ShowLoadingScreen (.AsBP%20Game%20Instance%201 (Utilities|Casting|CastToBP_GameInstance1 (Game|GetGameInstance)))))

(event Custom|ShowMainMenu
  (bind _returnvalue (Game|GetPlayerController 0))
  (bind _returnvalue_2 (UserInterface|CreateWidget "/Game/MultiplayerGame/Blueprints/Widget/MainMenu/6.6_C" _returnvalue))
  (UserInterface|Viewport|AddtoViewport _returnvalue_2 0)
  (Variables|/Script/Engine.PlayerController|SetbShowMouseCursor _returnvalue true))

(event Custom|ShowHostMenu
  (bind _returnvalue (UserInterface|CreateWidget "/Game/MultiplayerGame/Blueprints/Widget/MainMenu/5.5_C" (Game|GetPlayerController 0)))
  (UserInterface|Viewport|AddtoViewport _returnvalue 0))

(fn ConstructionScript)
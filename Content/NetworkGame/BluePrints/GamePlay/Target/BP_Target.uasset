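; BP_Target is a shootable target for a networked game that is randomly either Good or Bad.
; On BeginPlay the server picks the TargetState at 50/50 odds, and its RepNotify swaps the cone's material to match.
; When damaged by a player controller, it adjusts that player's BP_RoomPlayerState score, penalizing Good hits and rewarding Bad ones, then destroys the damage causer and itself.
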(event EventBeginPlay
  (Networking|SwitchHasAuthority
    (:Authority
      (CallFunction|RandomSwitchState))))

(event Game|Damage|EventAnyDamage
  (params (Damage :type Float%20%28single-precision%29) (DamageType :type Damage%20Type%20Object%20Reference) (InstigatedBy :type Controller%20Object%20Reference) (DamageCauser :type Actor%20Object%20Reference))
  (bind _as玩家控制器 (Utilities|Casting|CastToPlayerController InstigatedBy))
  (bind _asbp_room_player_state (Utilities|Casting|CastToBP_RoomPlayerState (Variables|/Script/Engine.Controller|GetPlayerState _as玩家控制器)))
  (Default|UpdateScore _asbp_room_player_state (Utilities|Select :Index (Variables|Default|GetTargetState) :NewEnumerator0 -2.0 :NewEnumerator1 2.0))
  (Actor|DestroyActor DamageCauser)
  (Actor|DestroyActor))

(fn ConstructionScript
  (Rendering|Material|SetMaterial (Variables|Default|GetCone) 0 (Utilities|Select :Index (Variables|Default|GetTargetState) :Option%200 0 :Option%201 0)))

(fn OnRepTargetState
  (Rendering|Material|SetMaterial (Variables|Default|GetCone) 0 (Utilities|Select :Index (Variables|Default|GetTargetState) :NewEnumerator0 "/Game/NetworkGame/BluePrints/GamePlay/Target/MI_GoodTarget.MI_GoodTarget" :NewEnumerator1 "/Game/NetworkGame/BluePrints/GamePlay/Target/MI_BadTarget.MI_BadTarget")))

(fn RandomSwitchState
  (Variables|Default|SetTargetState (select (>= (Math|Random|RandomFloatinRange 0.0 1.0) 0.5) "NewEnumerator0" "NewEnumerator1")))
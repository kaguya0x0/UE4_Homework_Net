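; Game instance for the multiplayer game, providing shared UI, session exit and player profile persistence.
; Events spawn loading-screen and delayed message widgets and destroy the session when leaving.
; Network and travel errors convert their failure enum to text and route it into the message window.
; Profile functions check, save and load player info through a single save slot, with check and save updating a profile-created flag.
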(event Custom|ShowMessageWindow
  (params (Message :type Text))
  (Utilities|FlowControl|Delay 0.5)
  (bind _returnvalue (UserInterface|CreateWidget "/Game/MultiplayerGame/Blueprints/Widget/General/2.2_C" (Game|GetPlayerController 0) Message))
  (UserInterface|Viewport|AddtoViewport _returnvalue 0))

(event Custom|LeaveGame
  (params (PlayerController :type Player%20Controller%20Object%20Reference))
  (|DestroySession PlayerController))

(event Custom|ShowLoadingScreen
  (bind _returnvalue (UserInterface|CreateWidget "/Game/MultiplayerGame/Blueprints/Widget/General/1.1_C" (Game|GetPlayerController 0)))
  (UserInterface|Viewport|AddtoViewport _returnvalue 0))

(event EventHandleNetworkError
  (params (FailureType :type ENetworkFailure%20Enum :default "NetDriverAlreadyExists") (bIsServer :type Boolean))
  (CallFunction|ShowMessageWindow (Utilities|Text|ToText(String) (Utilities|String|EnumtoString FailureType))))

(event EventHandleTravelError
  (params (FailureType :type ETravelFailure%20Enum :default "NoLevel"))
  (CallFunction|ShowMessageWindow (Utilities|Text|ToText(String) (Utilities|String|EnumtoString FailureType))))

(fn CheckSavedProfile
  (bind _returnvalue (SaveGame|DoesSaveGameExist (Variables|Profile|GetPlayerProfileName)))
  (bind _output_get (Variables|Profile|SetCreatedPlayerProfile _returnvalue))
  (return _output_get))

(fn SaveProfile
  (params (SaveGameObject :type BP%20Saved%20Player%20Profile%201%20Object%20Reference) (PlayerInfo :type 22%20Structure))
  (Variables|/Game/MultiplayerGame/Blueprints/General/BP_SavedPlayerProfile1.BP_SavedPlayerProfile1_C|SetSavedPlayerInfo SaveGameObject PlayerInfo)
  (bind _returnvalue (SaveGame|SaveGametoSlot SaveGameObject (Variables|Profile|GetPlayerProfileName)))
  (Variables|Profile|SetCreatedPlayerProfile _returnvalue))

(fn LoadProfile
  (bind _returnvalue (SaveGame|LoadGamefromSlot (Variables|Profile|GetPlayerProfileName)))
  (bind _asbp_saved_player_profile_1 (Utilities|Casting|CastToBP_SavedPlayerProfile1 _returnvalue))
  (return (Variables|/Game/MultiplayerGame/Blueprints/General/BP_SavedPlayerProfile1.BP_SavedPlayerProfile1_C|GetSavedPlayerInfo _asbp_saved_player_profile_1)))
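; Player controller for a multiplayer room that handles character spawning and in-game text chat.
; On local BeginPlay it clears widgets and passes PlayerInfo to an update event, which has BP_RoomGameMode1 respawn the chosen character class and creates the chat box.
; Chat messages fan out through the game mode's ConnectedPlayers to each controller's chat log.
; H toggles game-only and game-and-UI input; a GameInstance profile-loading branch is unconnected.
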(event Custom|CallServerUpdatePlayerInfo
  (params (PlayerInfo :type 22%20Structure))
  (Variables|Default|SetPlayerInfo PlayerInfo)
  (bind _asbp_room_game_mode_1 (Utilities|Casting|CastToBP_RoomGameMode1 (Game|GetGameMode)))
  (Default|RespawnCharacter _asbp_room_game_mode_1 self (.characterclass (Variables|Default|GetPlayerInfo)))
  (CallFunction|CreateGameplayChatBox))

(event Custom|ShowMapTime
  (params (MapTime :type Text))
  (Development|PrintText MapTime true true "(R=1.000000,G=0.000000,B=0.000000,A=1.000000)" 3e+01))

(event Custom|UpdateChatMessage
  (params (TextToSend :type Text))
  (Variables|Default|SetSendText TextToSend)
  (Variables|Default|SetSenderName (.name (Variables|Default|GetPlayerInfo)))
  (bind _asbp_room_game_mode_1 (Utilities|Casting|CastToBP_RoomGameMode1 (Game|GetGameMode)))
  (for _array_element (Variables|/Game/MultiplayerGame/Blueprints/Gameplay/BP_RoomGameMode1.BP_RoomGameMode1_C|GetConnectedPlayers _asbp_room_game_mode_1)
    (bind _asbp_room_player_controller_1 (Utilities|Casting|CastToBP_RoomPlayerController1 _array_element))
    (CallFunction|OnReceiveChatMessage _asbp_room_player_controller_1 (Variables|Default|GetSenderName) (Variables|Default|GetSendText))))

(event Custom|OnReceiveChatMessage
  (params (Sender :type Text) (Message :type Text))
  (Default|UpdateChatLog (Variables|/Game/NetworkGame/BluePrints/Wigets/GamePlay/WBP_ChatBox_Gameplay.WBP_ChatBox_Gameplay_C|GetGameplayChatBox (Variables|Default|GetGameplayChatBoxRef)) Sender Message))

(event Custom|CreateGameplayChatBox
  (bind _returnvalue (UserInterface|CreateWidget "/Game/NetworkGame/BluePrints/Wigets/GamePlay/WBP_ChatBox_Gameplay.WBP_ChatBox_Gameplay_C"))
  (bind _output_get (Variables|Default|SetGameplayChatBoxRef _returnvalue))
  (UserInterface|Viewport|AddtoViewport _output_get 0)
  (Variables|Default|SetbShowMouseCursor true))

(event EventBeginPlay
  (if (Pawn|IsLocalController)
    (Viewport|RemoveAllWidgets)
    (CallFunction|CallServerUpdatePlayerInfo (Variables|Default|GetPlayerInfo))))

(event Input|KeyboardEvents|H
  (params (Key :type Key%20Structure :default "None"))
  (bind _self self)
  (:Pressed
    (Utilities|FlowControl|FlipFlop
      (:A
        (Input|SetInputModeGameOnly _self)
        (Variables|Default|SetbShowMouseCursor true))
      (:B
        (Input|SetInputModeGameandUI _self (Variables|Default|GetGameplayChatBoxRef) "DoNotLock" true)
        (Variables|Default|SetbShowMouseCursor true)))))

(fn ConstructionScript)
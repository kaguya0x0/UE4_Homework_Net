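; Player controller for the multiplayer lobby, handling the lobby menu, player profile, character selection, chat and kicks.
; It loads or creates a saved profile, then passes player info to the lobby GameMode, which swaps characters and updates clients.
; Selection claims and frees slots in the GameMode's availability array, with index 0 always selectable.
; GameMode-driven events refresh the widget, chat relays through all connected controllers, and H toggles menu windows and input mode.
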(event Custom|Kicked
  (params (KickReason :type Text))
  (bind _returnvalue (Game|GetGameInstance))
  (bind _asbp_game_instance_1 (Utilities|Casting|CastToBP_GameInstance1 _returnvalue))
  (Utilities|FlowControl|Sequence
    (:then_0
      (Default|LeaveGame _asbp_game_instance_1 self))
    (:then_1
      (Default|ShowMessageWindow _asbp_game_instance_1 KickReason))
    (:then_2
      (Game|OpenLevel(byName) "MainMenu"))))

(event Custom|InitialPlayerInfo
  (CallFunction|UpdateSavedProfile)
  (CallFunction|CallServerUpdatePlayerInfo (Variables|Default|GetPlayerInfo) true))

(event Custom|UpdateCharacterInfo
  (params (CharacterClass :type BP%20Base%20Character%201%20Class%20Reference) (CharacterImage :type Texture%202D%20Object%20Reference))
  (bind _structout (Utilities|Struct|Setmembersin22 (Variables|Default|GetPlayerInfo) CharacterClass CharacterImage))
  (bind _returnvalue (SaveGame|CreateSaveGameObject "/Game/MultiplayerGame/Blueprints/General/BP_SavedPlayerProfile1.BP_SavedPlayerProfile1_C"))
  (Default|SaveProfile (.AsBP%20Game%20Instance%201 (Utilities|Casting|CastToBP_GameInstance1 (Game|GetGameInstance))) _returnvalue _structout)
  (CallFunction|CallServerUpdatePlayerInfo (Variables|Default|GetPlayerInfo) true))

(event Custom|UpdateChatMessage
  (params (TextToSend :type Text))
  (Variables|Default|SetSendText TextToSend)
  (Variables|Default|SetSenderName (.name (Variables|Default|GetPlayerInfo)))
  (bind _as1lobby_game_mode_1 (Utilities|Casting|CastTo1LobbyGameMode1 (Game|GetGameMode)))
  (for _array_element (Variables|/Game/MultiplayerGame/Blueprints/Lobby/1LobbyGameMode1.1LobbyGameMode1_C|GetConnectedPlayers _as1lobby_game_mode_1)
    (bind _asbp_lobby_player_controller_1 (Utilities|Casting|CastTo1LobbyPlayerController1 _array_element))
    (CallFunction|OnReceiveChatMessage _asbp_lobby_player_controller_1 (Variables|Default|GetSenderName) (Variables|Default|GetSendText))))

(event Custom|OnReceiveChatMessage
  (params (Sender :type Text) (Message :type Text))
  (Default|UpdateChatLog (Variables|/Game/NetworkGame/BluePrints/Wigets/Lobby/WBP_LobbyMenu.WBP_LobbyMenu_C|GetChatBoxWindow (Variables|Default|GetLobbyMenuRef)) Sender Message))

(event Custom|CallServerUpdatePlayerInfo
  (params (PlayerInfo :type 22%20Structure) (NeedSwapCharacter :type Boolean))
  (bind _output_get (Variables|Default|SetPlayerInfo PlayerInfo))
  (bind _as1lobby_game_mode_1 (Utilities|Casting|CastTo1LobbyGameMode1 (Game|GetGameMode)))
  (if NeedSwapCharacter
    (Default|SwapCharacter _as1lobby_game_mode_1 self (.characterclass _output_get)))
  (Default|UpdateClients _as1lobby_game_mode_1))

(event Custom|CreateLobbyMenu
  (params (ServerName :type Text))
  (Variables|Default|SetbShowMouseCursor true)
  (bind _returnvalue (UserInterface|CreateWidget "/Game/NetworkGame/BluePrints/Wigets/Lobby/WBP_LobbyMenu.WBP_LobbyMenu_C" self (Utilities|Text|ToText(String) (Utilities|String|Append "Server Name: " (Utilities|String|ToString(Text) ServerName)))))
  (bind _output_get (Variables|Default|SetLobbyMenuRef _returnvalue))
  (UserInterface|Viewport|AddtoViewport _output_get 0)
  (Input|SetInputModeGameandUI self _output_get "DoNotLock" true))

(event Custom|SelectCharacter
  (params (CharacterIndex :type Integer) (CharacterImage :type Texture%202D%20Object%20Reference))
  (bind _returnvalue (Game|GetGameMode))
  (bind _as1lobby_game_mode_1 (Utilities|Casting|CastTo1LobbyGameMode1 _returnvalue))
  (bind _availablecharacters (Variables|/Game/MultiplayerGame/Blueprints/Lobby/1LobbyGameMode1.1LobbyGameMode1_C|GetAvailableCharacters _as1lobby_game_mode_1))
  (Variables|Default|SetPreviousSelectCharacterIndex (Variables|Default|GetCurrentSelectCharacterIndex))
  (Variables|Default|SetCurrentSelectCharacterIndex CharacterIndex)
  (Variables|Default|SetCurrentSelectCharacterImage CharacterImage)
  (if (== 0 (Variables|Default|GetCurrentSelectCharacterIndex))
    (Utilities|Array|SetArrayElem _availablecharacters (Variables|Default|GetPreviousSelectCharacterIndex) true :!label _label)
    (CallFunction|UpdateCharacterInfo (Utilities|Array|Get(acopy) (Variables|/Game/MultiplayerGame/Blueprints/Lobby/1LobbyGameMode1.1LobbyGameMode1_C|GetCharactersClass _as1lobby_game_mode_1) (Variables|Default|GetCurrentSelectCharacterIndex)) (Variables|Default|GetCurrentSelectCharacterImage))
    (elif (not (Math|Boolean|Equal(Boolean) (Utilities|Array|Get(acopy) _availablecharacters (Variables|Default|GetCurrentSelectCharacterIndex)) false))
      (Utilities|Array|SetArrayElem _availablecharacters (Variables|Default|GetCurrentSelectCharacterIndex) false)
      (goto _label))))

(event Custom|UpdateLobbySettings
  (params (MapImage :type Texture%202D%20Object%20Reference) (MapName :type Text) (MapTime :type Text))
  (bind _lobbymenuref (Variables|Default|GetLobbyMenuRef))
  (Utilities|IsValid _lobbymenuref
    (:Is%20Valid
      (Variables|/Game/NetworkGame/BluePrints/Wigets/Lobby/WBP_LobbyMenu.WBP_LobbyMenu_C|SetMapTexture _lobbymenuref MapImage)
      (Variables|/Game/NetworkGame/BluePrints/Wigets/Lobby/WBP_LobbyMenu.WBP_LobbyMenu_C|SetMapName _lobbymenuref MapName)
      (Variables|/Game/NetworkGame/BluePrints/Wigets/Lobby/WBP_LobbyMenu.WBP_LobbyMenu_C|SetMapTime _lobbymenuref MapTime))))

(event Custom|UpdatePlayerNumDisplayText
  (params (CurrentPlayer :type Integer) (MaxPlayer :type Integer))
  (bind _lobbymenuref (Variables|Default|GetLobbyMenuRef))
  (Utilities|IsValid _lobbymenuref
    (:Is%20Valid
      (Variables|/Game/NetworkGame/BluePrints/Wigets/Lobby/WBP_LobbyMenu.WBP_LobbyMenu_C|SetPlayerNumDisplayText _lobbymenuref (Utilities|Text|ToText(String) (Utilities|String|Append (Utilities|String|ToString(Integer) CurrentPlayer) " of " (Utilities|String|ToString(Integer) MaxPlayer)))))))

(event Custom|UpdatePlayerInfoList
  (params (ConnectedPlayersInfo :type Array%20of%2022%20Structures))
  (bind _lobbymenuref (Variables|Default|GetLobbyMenuRef))
  (Utilities|IsValid _lobbymenuref
    (:Is%20Valid
      (Default|ClearPlayerInfoList _lobbymenuref)
      (for _array_element ConnectedPlayersInfo
        (Default|AddConnectedPlayerInfo _lobbymenuref _array_element)))))

(event Custom|UpdateAvailableCharacters
  (params (AvailableCharacters :type Array%20of%20Booleans))
  (bind _lobbymenuref (Variables|Default|GetLobbyMenuRef))
  (Utilities|IsValid _lobbymenuref
    (:Is%20Valid
      (for (_array_element _array_index) (Variables|/Game/NetworkGame/BluePrints/Wigets/Lobby/WBP_CharacterSelectWindow.WBP_CharacterSelectWindow_C|GetCharacterSelectButtons (Variables|/Game/NetworkGame/BluePrints/Wigets/Lobby/WBP_LobbyMenu.WBP_LobbyMenu_C|GetSelectCharacterWindow _lobbymenuref))
        (Widget|SetIsEnabled _array_element (Utilities|Array|Get(acopy) AvailableCharacters _array_index))))))

(event Custom|ShowLoadingScreen
  (Widget|RemovefromParent (Variables|Default|GetLobbyMenuRef))
  (Default|ShowLoadingScreen (.AsBP%20Game%20Instance%201 (Utilities|Casting|CastToBP_GameInstance1 (Game|GetGameInstance)))))

(event Input|KeyboardEvents|H
  (params (Key :type Key%20Structure :default "None"))
  (bind _self self)
  (bind _lobbymenuref (Variables|Default|GetLobbyMenuRef))
  (bind _lobbysettingswindow (Variables|/Game/NetworkGame/BluePrints/Wigets/Lobby/WBP_LobbyMenu.WBP_LobbyMenu_C|GetLobbySettingsWindow _lobbymenuref))
  (:Pressed
    (Utilities|FlowControl|FlipFlop
      (:A
        (Widget|SetVisibility _lobbysettingswindow "Hidden")
        (Input|SetInputModeGameOnly _self)
        (Variables|Default|SetbShowMouseCursor false))
      (:B
        (Widget|SetVisibility _lobbysettingswindow "Visible")
        (Input|SetInputModeGameandUI _self _lobbymenuref "DoNotLock" true)
        (Variables|Default|SetbShowMouseCursor true)))))

(fn ConstructionScript)

(fn UpdateSavedProfile
  (bind _returnvalue (Game|GetGameInstance))
  (bind _asbp_game_instance_1 (Utilities|Casting|CastToBP_GameInstance1 _returnvalue))
  (bind _doessavegameexist (Default|CheckSavedProfile _asbp_game_instance_1))
  (if _doessavegameexist
    (bind _savedplayerinfo (Default|LoadProfile _asbp_game_instance_1))
    (bind _returnvalue_2 (SaveGame|CreateSaveGameObject "/Game/MultiplayerGame/Blueprints/General/BP_SavedPlayerProfile1.BP_SavedPlayerProfile1_C"))
    (Utilities|Struct|Setmembersin22 (Variables|Default|GetPlayerInfo) (.Name (Utilities|Struct|Break22 _savedplayerinfo)) (.Avatar (Utilities|Struct|Break22 _savedplayerinfo)))
    (Default|SaveProfile _asbp_game_instance_1 _returnvalue_2 (Variables|Default|GetPlayerInfo))
    (else
      (bind _returnvalue_3 (SaveGame|CreateSaveGameObject "/Game/MultiplayerGame/Blueprints/General/BP_SavedPlayerProfile1.BP_SavedPlayerProfile1_C"))
      (Utilities|Struct|Setmembersin22 (Variables|Default|GetPlayerInfo) (Utilities|Text|ToText(String) (Utilities|String|Append "Player_" (.LeftS (Utilities|String|Split (Guid|ToString(Guid) (Guid|NewGuid)) "-")))))
      (Default|SaveProfile _asbp_game_instance_1 _returnvalue_3 (Variables|Default|GetPlayerInfo)))))